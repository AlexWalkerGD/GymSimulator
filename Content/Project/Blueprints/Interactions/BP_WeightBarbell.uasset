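; BP_WeightBarbell is a VR barbell actor meant to be held with two motion controllers.
; OnGrab stores first and second controllers based on an IsValid check, snapping the weight mesh to the first.
; With both valid, Tick sets actor rotation from a yaw-offset look-at between controllers, remapping pitch to roll and the first controller's roll to pitch.
; OnRelease is empty, so grabs are never cleared.
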(event `self.ReceiveBeginPlay`)

(event `/Game/Project/Blueprints/Interfaces/BPI_TwoHandsGrab.OnGrab`
  (params (MotionController :type "MotionControllerComponent Object Reference"))
  (`self.Motion Controller`
    (:`then`
      (set `self.SecondMotion Controller` MotionController))
    (:`else`
      (bind _output_get (set `self.Motion Controller` MotionController))
      (`SceneComponent.K2_AttachToComponent` (`self.SM_WeightDumbbell01_10LB`) _output_get "None" "SnapToTarget" "SnapToTarget" "KeepWorld" true))))

(event `/Game/Project/Blueprints/Interfaces/BPI_TwoHandsGrab.OnRelease`)

(event `self.ReceiveTick`
  (params (DeltaSeconds :type "Float (single-precision)"))
  (bind _motion_controller (`self.Motion Controller`))
  (bind _returnvalue_roll (`KismetMathLibrary.BreakRotator` (`SceneComponent.K2_GetComponentRotation` _motion_controller)))
  (bind (_returnvalue_roll_2 _returnvalue_pitch _returnvalue_yaw) (`KismetMathLibrary.BreakRotator` (`KismetMathLibrary.ComposeRotators` (`KismetMathLibrary.FindLookAtRotation` (`SceneComponent.K2_GetComponentLocation` _motion_controller) (`SceneComponent.K2_GetComponentLocation` (`self.SecondMotion Controller`))) (struct :`Yaw` -90.0))))
  (if (and (`KismetSystemLibrary.IsValid` (`self.Motion Controller`)) (`KismetSystemLibrary.IsValid` (`self.SecondMotion Controller`)))
    (`self.K2_SetActorRotation` (`KismetMathLibrary.MakeRotator` (* _returnvalue_pitch -1.0) _returnvalue_roll _returnvalue_yaw))))

(fn `UserConstructionScript`)